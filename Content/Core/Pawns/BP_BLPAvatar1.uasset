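; BP_BLPAvatar1 is an avatar pawn Blueprint with a Shape mesh, with no active logic in its event graph or construction script.
; An unconnected node chain casts the player state to BLPPlayerState and maps BLPPlayerId 0 to 3 to wide capsule, cone, sphere or torus meshes.
; That per-player shape selection never runs, as BeginPlay is empty and nothing triggers the chain.
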(event EventBeginPlay)

(fn ConstructionScript)