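; BP_BLPAvatar0 is a player avatar pawn Blueprint with a Shape mesh component, and it currently has no active logic.
; BeginPlay and the construction script are empty.
; A disconnected, never-executed chain would cast the PlayerState to BLPPlayerState and map BLPPlayerId 0 to 3 to a capsule, cone, sphere or torus mesh on Shape.
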(event EventBeginPlay)

(fn ConstructionScript)