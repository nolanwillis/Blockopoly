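; BP_BLPAvatar is a player avatar pawn Blueprint with a Shape mesh, currently without any active graph logic.
; BeginPlay and the construction script are empty.
; A disconnected chain would cast player state 0 to BLPPlayerState and pick a capsule, cone, sphere or torus mesh from BLPPlayerId, but it never runs.
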(event EventBeginPlay)

(fn ConstructionScript)