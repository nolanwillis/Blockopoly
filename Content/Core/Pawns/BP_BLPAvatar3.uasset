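; BP_BLPAvatar3 is an avatar pawn Blueprint with a Shape mesh component.
; Its event graph holds logic that would pick a capsule, cone, sphere or torus mesh from the BLPPlayerState's player ID.
; That logic is not wired to any event and never runs, as BeginPlay and the construction script are both empty.
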(event EventBeginPlay)

(fn ConstructionScript)