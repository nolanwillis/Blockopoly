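; BP_BLPAvatar2 is a player avatar Blueprint, kept with the core pawns, with a Shape mesh component.
; A disconnected event graph chain casts the PlayerState to BLPPlayerState and picks a wide capsule, cone, sphere or torus mesh from BLPPlayerId.
; That chain never runs, and both BeginPlay and the construction script are empty, so the Blueprint's graphs leave the shape unchanged.
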(event EventBeginPlay)

(fn ConstructionScript)