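; Estate property board space that labels itself with its name and price when play begins.
; SetupPropertyText runs ParseIntoArray on Name with an empty delimiter, putting the first element on Line1 and any second on Line2, otherwise blanking Line2.
; RentLine shows PurchaseCost with a dollar prefix, despite its rent naming.
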(event EventBeginPlay
  (CallFunction|SetupPropertyText))

(fn ConstructionScript)

(fn SetupPropertyText
  (bind _output_get (Variables|Default|SetNameArray (Utilities|String|ParseIntoArray (Variables|Default|GetName) " ")))
  (if (< (Utilities|Array|Length _output_get) 2)
    (Class|Text3DComponent|SetText (Variables|Default|GetLine1) (Utilities|Text|ToText(String) (Utilities|Array|Get(acopy) (Variables|Default|GetNameArray))))
    (Class|Text3DComponent|SetText (Variables|Default|GetLine2) (Utilities|Text|ToText(String) ""))
    (else
      (Class|Text3DComponent|SetText (Variables|Default|GetLine1) (Utilities|Text|ToText(String) (Utilities|Array|Get(acopy) (Variables|Default|GetNameArray))))
      (Class|Text3DComponent|SetText (Variables|Default|GetLine2) (Utilities|Text|ToText(String) (Utilities|Array|Get(acopy) (Variables|Default|GetNameArray) 1)))))
  (Class|Text3DComponent|SetText (Variables|Default|GetRentLine) (Utilities|Text|ToText(String) (Utilities|String|Append "$" (Utilities|String|ToString(Integer) (Variables|Default|GetPurchaseCost))))))