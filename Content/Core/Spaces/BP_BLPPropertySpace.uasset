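; Property space Blueprint that shows its name on two text elements, Line1 and Line2.
; On BeginPlay, SetupPropertyText parses the Name string into an array and assigns the first two entries to those lines.
; The parse delimiter is empty as stored, and both indices are read without a length check.
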(event EventBeginPlay
  (CallFunction|SetupPropertyText))

(fn ConstructionScript)

(fn SetupPropertyText
  (bind _name (Variables|Default|GetName))
  (bind _returnvalue (Utilities|String|ParseIntoArray _name " "))
  (Class|Text3DComponent|SetText (Variables|Default|GetLine1) (Utilities|Text|ToText(String) (Utilities|Array|Get(acopy) _returnvalue)))
  (Class|Text3DComponent|SetText (Variables|Default|GetLine2) (Utilities|Text|ToText(String) (Utilities|Array|Get(acopy) _returnvalue 1))))